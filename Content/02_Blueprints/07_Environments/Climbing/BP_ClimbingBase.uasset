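; BP_ClimbingBase is a climbable environment actor, apparently a base class, that marks where players can climb.
; Its CollisionBox overlap events run only on the server and filter for actors tagged Player.
; Begin overlap passes itself to the player through CanClimbMessage to enable climbing, and end overlap sends the same message to disable it.
; The climbing movement itself is not handled here.
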(event OnComponentBeginOverlap(CollisionBox)
  (params (OverlappedComponent :type Primitive%20Component%20Object%20Reference) (OtherActor :type Actor%20Object%20Reference) (OtherComp :type Primitive%20Component%20Object%20Reference) (OtherBodyIndex :type Integer) (bFromSweep :type Boolean) (SweepResult :type Hit%20Result%20Structure%20%28by%20ref%29))
  (Networking|SwitchHasAuthority
    (:Authority
      (if (Actor|ActorHasTag OtherActor "Player")
        (bind _player (Class|INTPlayerBase|GetPlayerRef(Message) OtherActor))
        (Class|INTPlayerBase|CanClimb(Message) _player self true)))))

(event OnComponentEndOverlap(CollisionBox)
  (params (OverlappedComponent :type Primitive%20Component%20Object%20Reference) (OtherActor :type Actor%20Object%20Reference) (OtherComp :type Primitive%20Component%20Object%20Reference) (OtherBodyIndex :type Integer))
  (Networking|SwitchHasAuthority
    (:Authority
      (if (Actor|ActorHasTag OtherActor "Player")
        (bind _player (Class|INTPlayerBase|GetPlayerRef(Message) OtherActor))
        (Class|INTPlayerBase|CanClimb(Message) _player 0 false)))))

(event EventBeginPlay)

(event Collision|EventActorBeginOverlap
  (params (OtherActor :type Actor%20Object%20Reference)))

(event EventTick
  (params (DeltaSeconds :type Float%20%28single-precision%29)))

(fn ConstructionScript)