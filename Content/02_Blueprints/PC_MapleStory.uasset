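; Player controller for a MapleStory-style game that handles character selection, spawning and possession.
; On BeginPlay, a client event creates and displays the character selection widget.
; Selecting a character passes the class and spawn location through a server event to the GameMode as a spawn request, using message-style calls.
; A separate SpawnPlayer event spawns the given class at a transform, adjusting for collisions, and possesses it.
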(event Custom|CL_InitializeWidgets
  ;[0.5 0 0.5] Initialize Widgets
  (bind _returnvalue (UserInterface|CreateWidget "/Game/04_UI/WB_CharacterSelection.WB_CharacterSelection_C"))
  (bind _output_get (Variables|Default|SetWB_CharacterSelection _returnvalue))
  (UserInterface|Viewport|AddtoViewport _output_get 0))

(event Custom|SRV_SelectCharacter
  (params (Player :type Actor%20Class%20Reference) (SpawnLocation :type Vector))
  ;[0.5 0 0.5] Select Character
  (bind _gamemode (Class|INTGameMode|GetGameModeRef(Message) (Game|GetGameMode)))
  (Class|INTGameMode|RequestSpawnPlayer(Message) _gamemode self Player SpawnLocation))

(event EventSelectCharacter
  (params (Player :type Actor%20Class%20Reference) (SpawnLocation :type Vector :default "0, 0, 0"))
  ;[0.5 0 0.5] Select Character
  (CallFunction|SRVSelectCharacter Player SpawnLocation))

(event EventSpawnPlayer
  (params (Player :type Actor%20Class%20Reference) (SpawnTransform :type Transform))
  ;[0.5 0 0.5] Spawn Player
  (bind _returnvalue (Game|SpawnActorfromClass Player SpawnTransform "AdjustIfPossibleButAlwaysSpawn" "MultiplyWithRoot" 0 0))
  (bind _player (Class|INTPlayerBase|GetPlayerRef(Message) _returnvalue))
  (Pawn|Possess _player))

(event EventBeginPlay
  (Utilities|FlowControl|Sequence
    (:then_0
      (CallFunction|InititailizeWidgets))))

(event EventInititailizeWidgets
  ;[0.5 0 0.5] Initialize Widgets
  (CallFunction|CLInitializeWidgets))

(fn ConstructionScript)

(fn GetPlayerControllerRef
  (return self))