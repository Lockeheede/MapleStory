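; Networked base player character for a MapleStory-style 2D Paper2D game, with side-scrolling walk, jump and rope climbing via Enhanced Input.
; Server RPCs set movement, climb and spawn state, and RepNotifies apply flipbooks, sprite facing, flying mode, collision type and location.
; A timer polls climb input while climbing is allowed, and jump sounds are multicast.
; A separately spawned camera actor trails the player using timer-driven timeline lerps, with a pause option.
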(event Custom|SRV_SetPlayerSpawnLocation
  ;[0.5 0 0.5] Set Spawn Location
  (bind _gamemode (Class|INTGameMode|GetGameModeRef(Message) (Game|GetGameMode)))
  (Variables|PlayerProperties|SetPlayerSpawnLocation (Variables|/Game/02_Blueprints/GM_MapleStory.GM_MapleStory_C|GetPlayerSpawnLocation _gamemode)))

(event Custom|UpdatePlayerCameraPosition
  ;[1 0.2 0] Update Follow Camera
  (bind _movementalpha (Timeline|PlayerCameraPosition PlayFromStart)
    (:Update
      (Transformation|SetActorLocation (Variables|PlayerCamera|GetPlayerCamera) (Math|Vector|Lerp(Vector) (Transformation|GetActorLocation (Variables|PlayerCamera|GetPlayerCamera)) (Variables|PlayerProperties|GetCurrentPlayerLocation) _movementalpha) false false))))

(event Custom|CL_PausePlayerCamera
  (params (Pause :type Boolean))
  (bind _getcurrentplayerlocationhandle (Variables|PlayerProperties|GetGetCurrentPlayerLocationHandle))
  ;[1 0.2 0] Update Follow Camera
  ;;[0 0 0] Pause Player Camera
  (if Pause
    (Utilities|Time|PauseTimerbyHandle _getcurrentplayerlocationhandle)
    (else
      (Utilities|Time|UnpauseTimerbyHandle _getcurrentplayerlocationhandle))))

(event EventBeginPlay
  ;[1 0 0] Begin Play
  (Utilities|FlowControl|Sequence
    (:then_0
      ;[1 0.2 0] Init
      (bind _aspc_maple_story (Utilities|Casting|CastToPC_MapleStory (Pawn|GetController)))
      (Utilities|IsValid (PlayerController|LocalPlayerSubsystems|GetEnhancedInputLocalPlayerSubsystem _aspc_maple_story)
        (:Is%20Valid
          (Input|AddMappingContext (PlayerController|LocalPlayerSubsystems|GetEnhancedInputLocalPlayerSubsystem _aspc_maple_story) "/Game/02_Blueprints/02_Inputs/IMC_Default.IMC_Default" 0 "(bIgnoreAllPressedKeysUntilRelease=True,bForceImmediately=False)"))))
    (:then_1
      ;[1 0.2 0] Spawn Camera
      (CallFunction|SetPlayerSpawnLocation)
      (Utilities|FlowControl|Delay 0.05)
      (bind _returnvalue (Game|SpawnActorfromClass "/Game/02_Blueprints/BP_Camera.BP_Camera_C" (Math|Transform|MakeTransform (Transformation|GetActorLocation)) "AdjustIfPossibleButAlwaysSpawn" "MultiplyWithRoot" 0 0))
      (Variables|PlayerCamera|SetPlayerCamera _returnvalue)
      (bind _playercontroller (Class|INTPlayerController|GetPlayerControllerRef(Message) (Pawn|GetController)))
      (Utilities|IsValid _playercontroller
        (:Is%20Valid
          (Game|Player|SetViewTargetwithBlend _playercontroller (Variables|PlayerCamera|GetPlayerCamera) 0.0 "VTBlend_Linear" 0.0 false)
          ;[1 0.2 0] Update Follow Camera
          (bind _returnvalue_2 (Utilities|Time|SetTimerbyEvent (delegate Custom|UpdatePlayerCameraPosition) 0.03 true))
          (Variables|PlayerProperties|SetUpdatePlayerCameraPositionHandle _returnvalue_2)
          (bind _returnvalue_3 (Utilities|Time|SetTimerbyFunctionName 0 "f_GetCurrentPlayerLocation" 0.1 true))
          (Variables|PlayerProperties|SetGetCurrentPlayerLocationHandle _returnvalue_3))))))

(event EventSetPlayerSpawnLocation
  ;[0.5 0 0.5] Set Spawn Location
  (CallFunction|SRVSetPlayerSpawnLocation))

(event EventPossessed
  (params (NewController :type Controller%20Object%20Reference))
  ;[0.5 0 0.5] To Work on Server
  ;[1 0.2 0] Init
  (bind _aspc_maple_story (Utilities|Casting|CastToPC_MapleStory (Pawn|GetController)))
  (Utilities|IsValid (PlayerController|LocalPlayerSubsystems|GetEnhancedInputLocalPlayerSubsystem _aspc_maple_story)
    (:Is%20Valid
      (Input|AddMappingContext (PlayerController|LocalPlayerSubsystems|GetEnhancedInputLocalPlayerSubsystem _aspc_maple_story) "/Game/02_Blueprints/02_Inputs/IMC_Default.IMC_Default" 0 "(bIgnoreAllPressedKeysUntilRelease=True,bForceImmediately=False)"))))

(event EventPausePlayerCamera
  (params (Pause :type Boolean))
  ;[1 0.2 0] Update Follow Camera
  ;;[0 0 0] Pause Player Camera
  (CallFunction|CLPausePlayerCamera Pause))

(event Custom|SRV_CanClimb
  (params (ClimbingObject :type Paper%20Sprite%20Actor%20Object%20Reference) (CanClimb :type Boolean))
  ;[1 1 0] Climbing
  (Variables|Climbing|SetClimbingObject ClimbingObject)
  (bind _output_get (Variables|Climbing|SetbCanClimb CanClimb))
  (if _output_get
    (bind _returnvalue (Utilities|Time|SetTimerbyEvent (delegate Custom|ClimbInput) 0.1 true))
    (Variables|Climbing|SetCheckClimbInputHandle _returnvalue)
    (elif (Variables|Climbing|GetbIsClimbing)
      (CallFunction|SetIsClimbing false)
      (else
        (Utilities|Time|ClearandInvalidateTimerbyHandle (Variables|Climbing|GetCheckClimbInputHandle))))))

(event Custom|SRV_SetMovementState
  (params (MovementState :type E_MovementState%20Enum :default "NewEnumerator0"))
  ;[1 0.8 0] Moving
  ;;[0 0 0] Server: Set Movement State
  (Variables|PlayerMovement|SetMovementState MovementState))

(event Custom|MC_Jump
  (params (JumpSFX :type Sound%20Base%20Object%20Reference) (PlayerLocation :type Vector))
  ;[0 1 0] Jumping
  ;;[0 0 0] Server Jump
  (Audio|PlaySoundatLocation JumpSFX PlayerLocation "0, 0, 0" 1.0 1.0 0.0 0 0 0 0))

(event Custom|SRV_Jump
  (params (JumpSFX :type Sound%20Base%20Object%20Reference) (PlayerLocation :type Vector))
  ;[0 1 0] Jumping
  ;;[0 0 0] Server Jump
  (CallFunction|MCJump JumpSFX PlayerLocation))

(event Custom|SRV_SetZAxisValue
  (params (ZAxis :type Float%20%28double-precision%29))
  ;[1 1 0] Climbing
  (Variables|PlayerMovement|SetZAxis ZAxis))

(event Custom|SRV_SetIsClimbing
  (params (bIsClimbing :type Boolean))
  ;[1 1 0] Climbing
  (Variables|Climbing|SetbIsClimbing bIsClimbing))

(event Custom|ClimbInput
  (bind _zaxis (Variables|PlayerMovement|GetZAxis))
  ;[1 1 0] Climbing
  (if (or (< _zaxis 0.0) (and (> _zaxis 0.0) (Variables|Climbing|GetbCanClimbUp)))
    (Utilities|Time|ClearandInvalidateTimerbyHandle (Variables|Climbing|GetCheckClimbInputHandle))
    (CallFunction|SetIsClimbing true)))

(event Custom|SRV_AdjustClimbingLocation
  (bind _returnvalue (Transformation|GetActorLocation))
  (bind (_x _y _z) (Math|Vector|BreakVector _returnvalue))
  ;[1 1 0] Climbing
  (bind _climbingobject (Variables|Climbing|GetClimbingObject)
    (:then
      (Variables|Climbing|SetClimbingLocation (Math|Vector|MakeVector (.X (Math|Vector|BreakVector (Transformation|GetActorLocation _climbingobject))) _y _z)))
    (:else)))

(event Custom|SRV_SetCanClimbUp
  (params (bCanClimbUp :type Boolean))
  ;[1 1 0] Climbing
  (Variables|Climbing|SetbCanClimbUp bCanClimbUp))

(event Custom|SRV_PauseClimbFlipbook
  (params (bPauseClimbFlipbook :type Boolean))
  ;[1 1 0] Climbing
  (Variables|Climbing|SetbPauseClimbFlipbook bPauseClimbFlipbook))

(event Input|EnhancedActionEvents|EnhancedInputActionIA_MoveRight
  (params (ActionValue :type Float%20%28double-precision%29) (ElapsedSeconds :type Float%20%28double-precision%29) (TriggeredSeconds :type Float%20%28double-precision%29) (InputAction :type Input%20Action%20Object%20Reference :default "/Game/02_Blueprints/02_Inputs/IA_MoveRight.IA_MoveRight"))
  ;[1 0.8 0] Moving
  (:Triggered
    (if (not (Variables|Climbing|GetbIsClimbing))
      (Pawn|Input|AddMovementInput (Math|Vector|GetForwardVector (Pawn|GetControlRotation :!class /Script/Engine.Pawn)) ActionValue false)
      (if (CallFunction|FIsNotJumping)
        (if (> ActionValue 0.0)
          (CallFunction|SetMovementState "NewEnumerator1")
          (else
            (CallFunction|SetMovementState "NewEnumerator2")))
        (else
          (CallFunction|SetMovementState "NewEnumerator3" :!label _label)))))
  (:Completed
    (if (not (Variables|Climbing|GetbIsClimbing))
      (if (CallFunction|FIsNotJumping)
        (CallFunction|SetMovementState "NewEnumerator0")
        (else
          (goto _label))))))

(event Input|EnhancedActionEvents|EnhancedInputActionIA_Jump
  (params (ActionValue :type Boolean) (ElapsedSeconds :type Float%20%28double-precision%29) (TriggeredSeconds :type Float%20%28double-precision%29) (InputAction :type Input%20Action%20Object%20Reference :default "/Game/02_Blueprints/02_Inputs/IA_Jump.IA_Jump"))
  ;[0 1 0] Jumping
  (:Triggered
    (if (and (CallFunction|FIsNotJumping) (not (Variables|Climbing|GetbIsClimbing)))
      (Character|Jump)
      (CallFunction|SRVJump (.JumpSFX (Utilities|Struct|BreakST_PlayerInfo (Variables|PlayerProperties|GetPlayerInfo))) (Transformation|GetActorLocation))
      (if (or (> (.Z (Math|Vector|BreakVector (Transformation|GetVelocity))) 0.0) (CallFunction|FIsNotJumping))
        (CallFunction|SetMovementState "NewEnumerator4")
        (else
          (CallFunction|SetMovementState "NewEnumerator3")))))
  (:Completed
    (Character|StopJumping)))

(event Input|EnhancedActionEvents|EnhancedInputActionIA_MoveUp
  (params (ActionValue :type Float%20%28double-precision%29) (ElapsedSeconds :type Float%20%28double-precision%29) (TriggeredSeconds :type Float%20%28double-precision%29) (InputAction :type Input%20Action%20Object%20Reference :default "/Game/02_Blueprints/02_Inputs/IA_MoveUp.IA_MoveUp"))
  ;[1 1 0] Climbing
  (:Triggered
    (if (Variables|Climbing|GetbCanClimb)
      (CallFunction|SetZAxisValue ActionValue)
      (Pawn|Input|AddMovementInput (Math|Vector|GetUpVector (Pawn|GetControlRotation :!class /Script/Engine.Pawn)) ActionValue false)
      (if (Variables|Climbing|GetbIsClimbing)
        (if (and (!= (Variables|PlayerMovement|GetZAxis) 0.0) (not (Audio|Components|Audio|IsPlaying (Variables|Default|GetSprite))))
          (CallFunction|PauseClimbFlipbook false)
          (else
            (if (and (== (Variables|PlayerMovement|GetZAxis) 0.0) (Audio|Components|Audio|IsPlaying (Variables|Default|GetSprite))) :!label _label
              (CallFunction|PauseClimbFlipbook true)
              (else
                (bind _climbingobject (Variables|Climbing|GetClimbingObject)
                  (:then
                    (if (!= (.X (Math|Vector|BreakVector (Transformation|GetActorLocation _climbingobject))) (.X (Math|Vector|BreakVector (Transformation|GetActorLocation))))
                      _))
                  (:else)))))))))
  (:Completed
    (CallFunction|SetZAxisValue ActionValue)
    (goto _label)))

(event EventOnLanded
  (params (Hit :type Hit%20Result%20Structure%20%28by%20ref%29))
  ;[0 1 0] Jumping
  ;;[0 0 0] Landing
  (CallFunction|SetMovementState "NewEnumerator0"))

(event EventSetMovementState
  (params (MovementState :type E_MovementState%20Enum :default "NewEnumerator0"))
  ;[1 0.8 0] Moving
  ;;[0 0 0] Server: Set Movement State
  (CallFunction|SRVSetMovementState MovementState))

(event EventCanClimb
  (params (ClimbingObject :type Paper%20Sprite%20Actor%20Object%20Reference) (bCanClimb :type Boolean))
  ;[1 1 0] Climbing
  (CallFunction|SRVCanClimb ClimbingObject bCanClimb))

(event EventSetZAxisValue
  (params (ZAxis :type Float%20%28double-precision%29))
  ;[1 1 0] Climbing
  (CallFunction|SRVSetZAxisValue ZAxis))

(event EventSetIsClimbing
  (params (bIsClimbing :type Boolean))
  ;[1 1 0] Climbing
  (CallFunction|SRVSetIsClimbing bIsClimbing))

(event EventAdjustClimbingLocation
  ;[1 1 0] Climbing
  (CallFunction|SRVAdjustClimbingLocation))

(event EventSetCanClimbUp
  (params (bCanClimbUp :type Boolean))
  ;[1 1 0] Climbing
  (CallFunction|SRVSetCanClimbUp bCanClimbUp))

(event EventPauseClimbFlipbook
  (params (bPauseClimbFlipbook :type Boolean))
  ;[1 1 0] Climbing
  (CallFunction|SRVPauseClimbFlipbook bPauseClimbFlipbook))

(fn ConstructionScript
  (|CallParentFunction))

(fn FIsNotJumping
  (return (not (AI|Components|NavMovement|IsFalling (Variables|Character|GetCharacterMovement)))))

(fn OnRepMovementState
  (bind _playerinfo (Variables|PlayerProperties|GetPlayerInfo))
  (bind (_idleanimation _movinganimation _jumpinganimation _fallinganimation) (Utilities|Struct|BreakST_PlayerInfo _playerinfo))
  (switch Utilities|FlowControl|Switch|SwitchonE_MovementState (Variables|PlayerMovement|GetMovementState)
    (:NewEnumerator0
      (Sprite|SetFlipbook (Variables|Default|GetSprite) _idleanimation))
    (:NewEnumerator1
      (Sprite|SetFlipbook (Variables|Default|GetSprite) _movinganimation)
      (Transformation|SetRelativeRotation (Variables|Default|GetSprite) "0, 0, 0" false false))
    (:NewEnumerator2
      (Sprite|SetFlipbook (Variables|Default|GetSprite) _movinganimation)
      (Transformation|SetRelativeRotation (Variables|Default|GetSprite) "0.000000,180.000000,0.000000" false false))
    (:NewEnumerator3
      (Sprite|SetFlipbook (Variables|Default|GetSprite) _jumpinganimation))
    (:NewEnumerator4
      (Sprite|SetFlipbook (Variables|Default|GetSprite) _fallinganimation))))

(fn OnRepPlayerSpawnLocation
  (Transformation|SetActorLocation (Variables|PlayerProperties|GetPlayerSpawnLocation) false false))

(fn FGetCurrentPlayerLocation
  (Variables|PlayerProperties|SetCurrentPlayerLocation (Transformation|GetActorLocation)))

(fn OnRepBIsClimbing
  (if (Variables|Climbing|GetbIsClimbing)
    (Pawn|Components|CharacterMovement|SetMovementMode (Variables|Character|GetCharacterMovement) "MOVE_Flying" 0)
    (Collision|SetCollisionObjectType (Variables|Default|GetCapsuleComponent) "ECC_GameTraceChannel1")
    (Sprite|SetFlipbook (Variables|Default|GetSprite) (Utilities|Struct|BreakST_PlayerInfo (Variables|PlayerProperties|GetPlayerInfo)))
    (else
      (Pawn|Components|CharacterMovement|SetMovementMode (Variables|Character|GetCharacterMovement) "MOVE_Falling" 0)
      (Collision|SetCollisionObjectType (Variables|Default|GetCapsuleComponent) "ECC_Pawn")
      (Sprite|SetFlipbook (Variables|Default|GetSprite) (Utilities|Struct|BreakST_PlayerInfo (Variables|PlayerProperties|GetPlayerInfo))))))

(fn OnRepClimbingLocation
  (Transformation|SetActorLocation (Variables|Climbing|GetClimbingLocation) false false))

(fn OnRepBPauseClimbFlipbook
  (bind _sprite (Variables|Default|GetSprite))
  (if (Variables|Climbing|GetbPauseClimbFlipbook)
    (Audio|Components|Audio|Stop _sprite)
    (else
      (Audio|Components|Audio|Play _sprite))))

(fn GetPlayerRef
  (bind _self self)
  (Utilities|IsValid _self
    (:Is%20Valid
      (return _self))))